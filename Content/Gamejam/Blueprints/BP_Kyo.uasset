(event `self.ReceiveBeginPlay`
  (bind _asplayer_controller (cast `PlayerController` (`self.GetController`)))
  (set `PlayerController.bShowMouseCursor` true _asplayer_controller)
  (`EnhancedInputSubsystemInterface.AddMappingContext` (pcsubsystem `EnhancedInputLocalPlayerSubsystem` _asplayer_controller) "/Game/Gamejam/Input/IMC_TopDown.IMC_TopDown" 0 (struct))
  (bind _returnvalue (`|CreateWidget` "/Game/Gamejam/UI/WBP_Start.WBP_Start_C"))
  (`UserWidget.AddToViewport` _returnvalue 0)
  (set `self.StartingUI` _returnvalue)
  (bind _returnvalue_2 (`|CreateWidget` "/Game/Gamejam/UI/WBP_Upgrade.WBP_Upgrade_C"))
  (set `/Game/Gamejam/UI/WBP_Upgrade.Kyo` self _returnvalue_2)
  (`UserWidget.AddToViewport` _returnvalue_2 0)
  (bind _output_get (set `self.UpgradeMenu` _returnvalue_2))
  (`Widget.SetVisibility` _output_get "Collapsed"))

(event `self.ReceiveTick`
  (params (DeltaSeconds :type "Float (single-precision)"))
  (bind _returnvalue (`self.K2_GetActorLocation`))
  (bind (_returnvalue_roll _returnvalue_pitch _returnvalue_yaw) (`KismetMathLibrary.BreakRotator` (`KismetMathLibrary.FindLookAtRotation` _returnvalue (`self.K2_GetActorLocation` (`.ReturnValue` (`GameplayStatics.FindNearestActor` _returnvalue (`self.Enemies`)))))))
  (`/Engine/EditorBlueprintResources/StandardMacros.Gate` true :!label _label
    (:`Exit`
      (`|ExecutionSequence`
        (:`then_0`
          (`KismetSystemLibrary.Delay` (`self.SpawnDelay`))
          (`self.SpawnEnemies`)
          (`/Engine/EditorBlueprintResources/StandardMacros.DoOnce` false
            (:`Completed`
              (goto _label_2 :!via `Open`))))
        (:`then_1`
          (`/Engine/EditorBlueprintResources/StandardMacros.Gate` true :!label _label_2
            (:`Exit`
              (`|ExecutionSequence`
                (:`then_1`
                  (if (`self.MissileUnlock`)
                    (`KismetSystemLibrary.Delay` (`self.MissileDelay`))
                    (`|SpawnActorFromClass` "/Game/Gamejam/BP_Projectile_3_Small.BP_Projectile_3_Small_C" (`KismetMathLibrary.MakeTransform` (`SceneComponent.K2_GetComponentLocation` (`self.ProjectileEmitter`)) (`KismetMathLibrary.MakeRotator` _returnvalue_roll 0.0 _returnvalue_yaw) (0.2 0.2 0.2)) "AlwaysSpawn" "MultiplyWithRoot" null (`self.MissileDamage`) null)))))))))))

(event `EnhancedInput|/Game/Gamejam/Input/IA_Move`
  (params (ActionValue :type "Vector2D Structure") (ElapsedSeconds :type "Float (double-precision)") (TriggeredSeconds :type "Float (double-precision)") (InputAction :type "InputAction Object Reference" :default "/Game/Gamejam/Input/IA_Move.IA_Move"))
  (:`Triggered`
    (`self.AddMovementInput` (1.0 0.0 0.0) ActionValue_X)
    (`self.AddMovementInput` (0.0 -1.0 0.0) ActionValue_Y)
    (set `self.Directionality` (`KismetMathLibrary.MakeVector2D` ActionValue_X ActionValue_Y))
    (`/Engine/EditorBlueprintResources/StandardMacros.DoOnce` false
      (:`Completed`
        (`ActorComponent.ToggleActive` (`self.NS_GoldenCreature`))
        (`ActorComponent.ToggleActive` (`self.NS_RunesVariation3`))
        (`KismetSystemLibrary.K2_SetTimerDelegate` (delegate `CultSpawn`) 120.0)
        (`Widget.RemoveFromParent` (`self.StartingUI`))
        (`KismetSystemLibrary.CollectGarbage`)
        (goto _label :!via `Open`))))
  (:`Started`
    (set `self.IsHoldingMove` true))
  (:`Completed`
    (set `self.IsHoldingMove` false)))

(event `CultSpawn`
  (set `self.ChosenEnemy` "NewEnumerator1")
  (`KismetSystemLibrary.K2_SetTimerDelegate` (delegate `DemonSpawn`) 60.0))

(event `DemonSpawn`
  (set `self.ChosenEnemy` "NewEnumerator2")
  (`KismetSystemLibrary.K2_SetTimerDelegate` (delegate `HarpieSpawn`) 60.0))

(event `self.ReceiveAnyDamage`
  (params (Damage :type "Float (single-precision)") (DamageType :type "DamageType Object Reference") (InstigatedBy :type "Controller Object Reference") (DamageCauser :type "Actor Object Reference"))
  (bind _output_get (set `self.CurrentHealth` (- (`self.CurrentHealth`) Damage)))
  (if (<= _output_get 0.0)
    (`self.Death`)
    (bind _p_health_bar (`self.P health bar`)
      (:`then`
        (`/Game/Gamejam/UI/PHealthBar.UpdateWidgetText` _p_health_bar 0.0))
      (:`else`))
    (else
      (bind _p_health_bar_2 (`self.P health bar` :!label _label_3)
        (:`then`
          (`/Game/Gamejam/UI/PHealthBar.UpdateWidgetText` _p_health_bar_2 (`self.CurrentHealth`)))
        (:`else`
          (bind _asphealth_bar (cast `/Game/Gamejam/UI/PHealthBar` (`WidgetComponent.GetWidget` (`self.WidgetText`))))
          (set `self.P health bar` _asphealth_bar)
          (goto _label_3))))))

(event `HarpieSpawn`
  (set `self.ChosenEnemy` "NewEnumerator4")
  (`KismetSystemLibrary.K2_SetTimerDelegate` (delegate `WolfSpawn`) 60.0))

(event `WolfSpawn`
  (set `self.ChosenEnemy` "NewEnumerator5")
  (`KismetSystemLibrary.K2_SetTimerDelegate` (delegate `KnightSpawn`) 60.0))

(event `KnightSpawn`
  (set `self.ChosenEnemy` "NewEnumerator3"))

(fn `CalculateHealth`
  (params (DamageReceived :type "Float (double-precision)"))
  (returns (HealthPercent :type "Float (double-precision)"))
  (return 0.0))

(fn `Death`
  (`GameplayStatics.SetGamePaused` true)
  (bind _returnvalue (`|CreateWidget` "/Game/Gamejam/UI/WBP_Death.WBP_Death_C"))
  (`UserWidget.AddToViewport` _returnvalue 0))

(fn `DestroyEnemy`
  (params (Enemy :type "/Game/Gamejam/Blueprints/BP_Enemy Object Reference"))
  (`KismetArrayLibrary.Array_RemoveItem` (`self.Enemies`) Enemy)
  (`self.K2_DestroyActor` Enemy)
  (`KismetSystemLibrary.CollectGarbage`)
  (bind _result (`/Engine/EditorBlueprintResources/StandardMacros.IncrementInt` (`self.KillCount`))
    (:`  `
      (if (== (mod _result (`self.LevelReq`)) 0)
        (set `self.KillCount` 0)
        (set `self.LevelReq` (`KismetMathLibrary.FFloor` (* (`KismetMathLibrary.Conv_IntToDouble` (`self.LevelReq`)) 1.2)))
        (`GameplayStatics.SetGamePaused` true)
        (`Widget.SetVisibility` (`self.UpgradeMenu`) "Visible")))))

(fn `IsStuck`
  (returns (IsStuck :type Boolean))
  (return (and (`self.IsHoldingMove`) (< (`KismetMathLibrary.VSize` (`self.GetVelocity`)) (`self.StuckThreshold`)))))

(fn `SpawnEnemies`
  (bind (_returnvalue_x _returnvalue_y) (`KismetMathLibrary.BreakVector` (`self.K2_GetActorLocation`)))
  (bind (_returnvalue_x_2 _returnvalue_y_2) (`KismetMathLibrary.BreakVector` (`KismetMathLibrary.RandomUnitVector`)))
  (bind _returnvalue (`|SpawnActorFromClass` (`BlueprintMapLibrary.Map_Find` (`self.EnemyMap`) (`self.ChosenEnemy`)) (`KismetMathLibrary.MakeTransform` (`KismetMathLibrary.MakeVector` (+ (* 1000.0 _returnvalue_x_2) _returnvalue_x) (+ (* 1000.0 _returnvalue_y_2) _returnvalue_y))) "Undefined" "MultiplyWithRoot" null null))
  (`/Engine/EditorBlueprintResources/StandardMacros.IsValid` _returnvalue
    (:`Is Valid`
      (bind _asbp_enemy (cast `/Game/Gamejam/Blueprints/BP_Enemy` _returnvalue))
      (set `/Game/Gamejam/Blueprints/BP_Enemy.Target` self _asbp_enemy)
      (`KismetArrayLibrary.Array_AddUnique` (`self.Enemies`) _asbp_enemy))))

(fn `UpgradeSelected`
  (set `CharacterMovementComponent.MaxWalkSpeed` (`self.MovementSpeed`) (`self.CharacterMovement`))
  (`Widget.SetVisibility` (`self.UpgradeMenu`) "Collapsed")
  (`GameplayStatics.SetGamePaused` false))

(fn `UserConstructionScript`)