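; BP_Enemy is a sprite-based enemy that chases a Target and deals contact damage to BP_Kyo when an overlap begins.
; Each Tick it writes the Target's location to the TargetLocation blackboard key for its AI.
; Damage lowers health and briefly swaps the sprite to a Flash material; after that delay, zero health hands destruction to the Target's DestroyEnemy.
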(event `self.ReceiveBeginPlay`
  (set `self.SpriteMat` (`PrimitiveComponent.GetMaterial` (`self.Sprite`) 0)))

(event `self.ReceiveTick`
  (params (DeltaSeconds :type "Float (single-precision)"))
  (`BlackboardComponent.SetValueAsVector` (`AIBlueprintHelperLibrary.GetBlackboard` null) "TargetLocation" (`self.K2_GetActorLocation` (`self.Target`))))

(event `self.ReceiveAnyDamage`
  (params (Damage :type "Float (single-precision)") (DamageType :type "DamageType Object Reference") (InstigatedBy :type "Controller Object Reference") (DamageCauser :type "Actor Object Reference"))
  (bind _output_get (set `self.CurrentHealth` (- (`self.CurrentHealth`) Damage)))
  (`PrimitiveComponent.SetMaterial` (`self.Sprite`) 0 "/Game/Gamejam/Flash.Flash")
  (`KismetSystemLibrary.Delay` 0.2)
  (`PrimitiveComponent.SetMaterial` (`self.Sprite`) 0 (`self.SpriteMat`))
  (if (<= _output_get 0.0)
    (`/Game/Gamejam/Blueprints/BP_Kyo.DestroyEnemy` (`self.Target`) self)))

(event `self.ReceiveActorBeginOverlap`
  (params (OtherActor :type "Actor Object Reference"))
  (bind _asbp_kyo (cast `/Game/Gamejam/Blueprints/BP_Kyo` OtherActor))
  (`GameplayStatics.ApplyDamage` _asbp_kyo (`self.Damage`)))

(fn `UserConstructionScript`)